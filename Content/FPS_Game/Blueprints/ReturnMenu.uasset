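; ReturnMenu is a trigger actor, likely a return-to-menu prompt, that tells the player character when it is in range.
; Box overlap begin and end set IsInRange on the overlapping BP_LPSP_PCH and mirror it in a local InTrigger flag.
; Both events then toggle the TextRender's visibility; the InTrigger branch runs the same toggle either way.
; No menu loading happens in this Blueprint.
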(event OnComponentBeginOverlap(Box)
  (params (OverlappedComponent :type Primitive%20Component%20Object%20Reference) (OtherActor :type Actor%20Object%20Reference) (OtherComp :type Primitive%20Component%20Object%20Reference) (OtherBodyIndex :type Integer) (bFromSweep :type Boolean) (SweepResult :type Hit%20Result%20Structure%20%28by%20ref%29))
  (bind _textrender (Variables|Default|GetTextRender))
  (bind _asbp_lpsp_pch (Utilities|Casting|CastToBP_LPSP_PCH OtherActor))
  (Variables|/LPSPSample/LPSPSample/Core/BP_LPSP_PCH.BP_LPSP_PCH_C|SetIs%20in%20range _asbp_lpsp_pch true)
  (Variables|Default|Setin%20trigger true)
  (if (Variables|Default|Getin%20trigger)
    (Rendering|ToggleVisibility _textrender false)
    (else
      (Rendering|ToggleVisibility _textrender false))))

(event OnComponentEndOverlap(Box)
  (params (OverlappedComponent :type Primitive%20Component%20Object%20Reference) (OtherActor :type Actor%20Object%20Reference) (OtherComp :type Primitive%20Component%20Object%20Reference) (OtherBodyIndex :type Integer))
  (bind _textrender (Variables|Default|GetTextRender))
  (bind _asbp_lpsp_pch (Utilities|Casting|CastToBP_LPSP_PCH OtherActor))
  (Variables|/LPSPSample/LPSPSample/Core/BP_LPSP_PCH.BP_LPSP_PCH_C|SetIs%20in%20range _asbp_lpsp_pch false)
  (Variables|Default|Setin%20trigger false)
  (if (Variables|Default|Getin%20trigger)
    (Rendering|ToggleVisibility _textrender false)
    (else
      (Rendering|ToggleVisibility _textrender false))))

(fn ConstructionScript)