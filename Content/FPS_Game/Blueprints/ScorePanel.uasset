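; Score panel actor that displays the player's shooting results: enemy kills, civilian kills, accuracy and time.
; Every Tick it casts player character 0 to BP_LPSP_PCH and reads its hit, shot and last-time counters.
; It formats them into four text fields, with hard-coded kill totals and accuracy computed as a rounded percentage of target hits over bullets shot.
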(event EventTick
  (params (DeltaSeconds :type Float%20%28single-precision%29))
  (bind _asbp_lpsp_pch (Utilities|Casting|CastToBP_LPSP_PCH (Game|GetPlayerCharacter 0)))
  (Variables|Default|SetCharacter%20REF _asbp_lpsp_pch)
  (Utilities|FlowControl|Sequence
    (:then_0
      ;[1 0.8011 0.2045] Target hit
      (Rendering|Components|TextRender|SetText (Variables|Default|GetKills%20text) (Utilities|Text|FormatText "Enemies killed: {kills} / 30" (Utilities|Text|ToText(Integer) (Variables|/LPSPSample/LPSPSample/Core/BP_LPSP_PCH.BP_LPSP_PCH_C|GetTarget%20hit%20count (Variables|Default|GetCharacter%20REF))))))
    (:then_1
      ;[1 0.8011 0.2045] Civilian hit
      (Rendering|Components|TextRender|SetText (Variables|Default|GetCivil%20text) (Utilities|Text|FormatText "Civilians killed: {kills} / 12" (Utilities|Text|ToText(Integer) (Variables|/LPSPSample/LPSPSample/Core/BP_LPSP_PCH.BP_LPSP_PCH_C|GetCivil%20hit%20count (Variables|Default|GetCharacter%20REF))))))
    (:then_2
      ;[1 0.8011 0.2045] Accuracy
      (Rendering|Components|TextRender|SetText (Variables|Default|GetAccuracy%20text) (Utilities|Text|FormatText "Accuracy: {accuracy}%" (Utilities|Text|ToText(Integer) (Math|Float|Round (* (/ (Math|Conversions|ToFloat(Integer) (Variables|/LPSPSample/LPSPSample/Core/BP_LPSP_PCH.BP_LPSP_PCH_C|GetScore:%20target%20hit (Variables|Default|GetCharacter%20REF))) (Math|Conversions|ToFloat(Integer) (Variables|/LPSPSample/LPSPSample/Core/BP_LPSP_PCH.BP_LPSP_PCH_C|GetScore:%20bullet%20shot (Variables|Default|GetCharacter%20REF)))) 1e+02))))))
    (:then_3
      ;[1 0.8011 0.2045] Timer
      (Rendering|Components|TextRender|SetText (Variables|Default|GetTimer%20text) (Utilities|Text|FormatText "Your time: {seconds}:{milliseconds}0 s" (Variables|/LPSPSample/LPSPSample/Core/BP_LPSP_PCH.BP_LPSP_PCH_C|GetTimer:%20last%20time%20%28s%29 (Variables|Default|GetCharacter%20REF)) (Variables|/LPSPSample/LPSPSample/Core/BP_LPSP_PCH.BP_LPSP_PCH_C|GetTimer:%20last%20time%20%28ms%29 (Variables|Default|GetCharacter%20REF)))))))

(fn ConstructionScript)