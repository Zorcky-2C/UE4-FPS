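; StartTimer is a one-shot trigger box that begins a timed target-shooting run with civilian targets.
; On first overlap it resets the player character's counters and activates all basic, moving, civilian and moving-civilian targets.
; It then creates the HUD widgets for timer, hit counter, accuracy and civilian count.
; Its StopTimer event stops the timer and removes those widgets from the screen.
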(event OnComponentBeginOverlap(Box)
  (params (OverlappedComponent :type Primitive%20Component%20Object%20Reference) (OtherActor :type Actor%20Object%20Reference) (OtherComp :type Primitive%20Component%20Object%20Reference) (OtherBodyIndex :type Integer) (bFromSweep :type Boolean) (SweepResult :type Hit%20Result%20Structure%20%28by%20ref%29))
  (if (not (Variables|Default|GetHas%20been%20triggered?))
    (Variables|Default|SetHas%20been%20triggered? true)
    ;[1 0.9279 0.2311] Reset player counters
    (bind _asbp_lpsp_pch (Utilities|Casting|CastToBP_LPSP_PCH (Game|GetPlayerCharacter 0)))
    (Default|ResetCounters _asbp_lpsp_pch)
    (Utilities|FlowControl|Sequence
      (:then_0
        (bind _outactors (Actor|GetAllActorsOfClass "/LPSPSample/LPSPSample/Core/Target_basic.Target_basic_C"))
        (Default|SetTargetActive _outactors))
      (:then_1
        (bind _outactors_2 (Actor|GetAllActorsOfClass "/LPSPSample/LPSPSample/Core/Target_moving.Target_moving_C"))
        (Default|SetTargetActive _outactors_2))
      (:then_2
        (bind _outactors_3 (Actor|GetAllActorsOfClass "/LPSPSample/LPSPSample/Core/Target_Civil.Target_Civil_C"))
        (Default|SetTargetActive _outactors_3))
      (:then_3
        (bind _outactors_4 (Actor|GetAllActorsOfClass "/LPSPSample/LPSPSample/Core/Target_civil_moving.Target_civil_moving_C"))
        (Default|SetTargetActive _outactors_4)
        ;[1 1 1] Timer
        (bind _returnvalue (UserInterface|CreateWidget "/Game/FPS_Game/Blueprints/Timer.Timer_C"))
        (bind _output_get (Variables|Default|SetTimer%20Ref _returnvalue))
        (UserInterface|Viewport|AddtoViewport _output_get 0)
        ;[1 0.8349 0.1142] Target hit counter
        (bind _returnvalue_2 (UserInterface|CreateWidget "/LPSPSample/LPSPSample/Core/TargerCounter.TargerCounter_C" (Game|GetPlayerController 0)))
        (UserInterface|Viewport|AddtoViewport _returnvalue_2 0)
        ;[1 0.8349 0.1142] Score
        (bind _returnvalue_3 (UserInterface|CreateWidget "/LPSPSample/LPSPSample/Core/Accuracy.Accuracy_C" (Game|GetPlayerController 0)))
        (UserInterface|Viewport|AddtoViewport _returnvalue_3 0)
        ;[1 0.8349 0.1142] Civils
        (bind _returnvalue_4 (UserInterface|CreateWidget "/LPSPSample/LPSPSample/Core/Civil_Counter.Civil_Counter_C" (Game|GetPlayerController 0)))
        (UserInterface|Viewport|AddtoViewport _returnvalue_4 0)))))

(event Custom|Stop%20Timer
  (Default|StopTimer (Variables|Default|GetTimer%20Ref))
  (Widget|RemovefromParent (stale OnComponentBeginOverlap(Box) _returnvalue))
  (Widget|RemovefromParent (stale OnComponentBeginOverlap(Box) _returnvalue_2))
  (Widget|RemovefromParent (stale OnComponentBeginOverlap(Box) _returnvalue_3))
  (Widget|RemovefromParent (stale OnComponentBeginOverlap(Box) _returnvalue_4)))

(fn ConstructionScript)